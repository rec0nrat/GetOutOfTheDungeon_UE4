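; Door actor that swings open and closed in response to open and close requests from its OpenDoor component.
; It stores its starting rotation at BeginPlay, then plays or reverses the OpenAnim timeline on each request.
; The timeline's SwingAngle, scaled by the component's OpenAngle, is subtracted from the initial yaw.
; When the timeline finishes, it toggles the component's IsOpen flag.
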(event `self.ReceiveBeginPlay`
  (set `self.InitialRotation` (`self.K2_GetActorRotation`)))

(event `self.OpenDoor.OnOpenRequest`
  (bind _opendoor (`self.OpenDoor`))
  (bind (_direction _swingangle) (`Timeline|OpenAnim` :!label _label)
    (:`Update`
      (`self.K2_SetActorRotation` (`KismetMathLibrary.MakeRotator` (.roll (`self.InitialRotation`)) (.pitch (`self.InitialRotation`)) (- (.yaw (`self.InitialRotation`)) (* _swingangle (`OpenDoor.OpenAngle` (`self.OpenDoor`)))))))
    (:`Finished`
      (set `OpenDoor.isOpen` (not (`OpenDoor.isOpen` _opendoor)) _opendoor))))

(event `self.OpenDoor.OnCloseRequest`
  (goto _label :!via `Reverse`))

(fn `UserConstructionScript`)